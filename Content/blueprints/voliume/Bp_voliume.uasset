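; Level-transition trigger volume that sends the player to MainLevel_2.
; When the player pawn overlaps its Box component, it counts the BPcrystal actors in the world.
; If any crystals exist, it opens the level after a short delay; if none remain, it only prints a debug "Hello".
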(event OnComponentBeginOverlap(Box)
  (params (OverlappedComponent :type Primitive%20Component%20Object%20Reference) (OtherActor :type Actor%20Object%20Reference) (OtherComp :type Primitive%20Component%20Object%20Reference) (OtherBodyIndex :type Integer) (bFromSweep :type Boolean) (SweepResult :type Hit%20Result%20Structure%20%28by%20ref%29))
  (Utilities|IsValid 0
    (:Is%20Valid
      (if (== OtherActor (Game|Player|GetPlayerPawn 0))
        (bind _outactors (Actor|GetAllActorsOfClass "/Game/blueprints/BP-crystal.BP-crystal_C"))
        (if (Math|Conversions|ToBoolean(Integer) (Utilities|Array|Length _outactors))
          (Utilities|FlowControl|Delay 0.2)
          (Game|OpenLevel(byName) "MainLevel_2")
          (else
            (Development|PrintString "Hello")))))))

(event EventBeginPlay)

(event Collision|EventActorBeginOverlap
  (params (OtherActor :type Actor%20Object%20Reference)))

(event EventTick
  (params (DeltaSeconds :type Float%20%28single-precision%29)))

(fn ConstructionScript)